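; BP_StandardEnemy is an enemy whose Blueprint logic drives an on-actor health display from its Ability System Component.
; Every Tick it casts the Widget component's user widget to WBP_HealthShow, then writes health and max health attributes into the text.
; The inner slider's X render scale follows the ratio of two attribute reads, acting as a health bar.
; When the checked attribute reaches zero or below, the text turns red; no death logic runs here.
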(event EventBeginPlay)

(event Collision|EventActorBeginOverlap
  (params (OtherActor :type Actor%20Object%20Reference)))

(event EventTick
  (params (DeltaSeconds :type Float%20%28single-precision%29))
  (bind _asc (Variables|Default|GetASC))
  (bind _returnvalue (Ability|Attribute|GetFloatAttributefromAbilitySystemComponent _asc "(AttributeName=\"Health\",Attribute=/Script/GAS_Exercice.GeneralStatsAttributeSet:Health,AttributeOwner=\"/Script/CoreUObject.Class'/Script/GAS_Exercice.GeneralStatsAttributeSet'\")"))
  (bind _returnvalue_2 (Ability|Attribute|GetFloatAttributefromAbilitySystemComponent _asc "(AttributeName=\"MaxHealth\",Attribute=/Script/GAS_Exercice.GeneralStatsAttributeSet:MaxHealth,AttributeOwner=\"/Script/CoreUObject.Class'/Script/GAS_Exercice.GeneralStatsAttributeSet'\")"))
  (bind _aswbp_health_show (Utilities|Casting|CastToWBP_HealthShow (UserInterface|GetUserWidgetObject (Variables|Default|GetWidget))))
  (Variables|/Script/UMG.TextBlock|SetText (Variables|/Game/CustomBlueprints/Widget/WBP_HealthShow.WBP_HealthShow_C|GetHealthText _aswbp_health_show) (Utilities|Text|FormatText "Health: {Health}/{MaxHealth}" _returnvalue _returnvalue_2))
  (Class|Widget|SetRenderTransform (Variables|/Game/CustomBlueprints/Widget/WBP_HealthShow.WBP_HealthShow_C|GetSlider_Inner _aswbp_health_show) (Utilities|Struct|MakeWidgetTransform (.translation (Variables|/Script/UMG.Widget|GetRenderTransform (Variables|/Game/CustomBlueprints/Widget/WBP_HealthShow.WBP_HealthShow_C|GetSlider_Inner _aswbp_health_show))) (Math|Vector2D|MakeVector2D (/ _returnvalue _returnvalue_2) (.y (.scale (Variables|/Script/UMG.Widget|GetRenderTransform (Variables|/Game/CustomBlueprints/Widget/WBP_HealthShow.WBP_HealthShow_C|GetSlider_Inner _aswbp_health_show))))) (.shear (Variables|/Script/UMG.Widget|GetRenderTransform (Variables|/Game/CustomBlueprints/Widget/WBP_HealthShow.WBP_HealthShow_C|GetSlider_Inner _aswbp_health_show))) (.angle (Variables|/Script/UMG.Widget|GetRenderTransform (Variables|/Game/CustomBlueprints/Widget/WBP_HealthShow.WBP_HealthShow_C|GetSlider_Inner _aswbp_health_show)))))
  (if (<= _returnvalue 0.0)
    (Appearance|SetColorandOpacity (Variables|/Game/CustomBlueprints/Widget/WBP_HealthShow.WBP_HealthShow_C|GetHealthText _aswbp_health_show) (Utilities|Struct|MakeSlateColor "(R=1.000000,G=0.000000,B=0.055699,A=1.000000)") :!class /Script/UMG.TextBlock)))

(fn ConstructionScript)